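; Game instance Blueprint that keeps the player's inventory, health and keys, in an SInventory struct.
; Functions add, consume, read and reset keys, with consumption returning whether enough keys were held.
; Damage lowers health no further than zero and, once it is depleted, calls Defeated on the IcaroBP player pawn.
; Reset functions restore full health or clear the key count.
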(fn AddKeys
  (params (NumKeys :type Integer))
  (Utilities|Struct|SetmembersinSInventory (Variables|Default|GetSInventory) (+ NumKeys (.Keys (Utilities|Struct|BreakSInventory (Variables|Default|GetSInventory)))))
  (return))

(fn ConsumeKeys
  (params (NumKeys :type Integer))
  (if (<= NumKeys (.Keys (Utilities|Struct|BreakSInventory (Variables|Default|GetSInventory))))
    (Utilities|Struct|SetmembersinSInventory (Variables|Default|GetSInventory) (- (.Keys (Utilities|Struct|BreakSInventory (Variables|Default|GetSInventory))) NumKeys))
    (return true)
    (else
      (return false))))

(fn ConsumeHealth
  (params (Damage :type Integer))
  (bind _sinventory (Variables|Default|GetSInventory))
  (bind _health (Utilities|Struct|BreakSInventory _sinventory))
  (bind _returnvalue (- _health Damage))
  (if (> _health 0)
    (if (>= _returnvalue 0)
      (Utilities|Struct|SetmembersinSInventory _sinventory _returnvalue)
      (else
        (Utilities|Struct|SetmembersinSInventory _sinventory 0)))
    (if (> _health 0)
      _
      (else
        (Default|Defeated (.AsIcaro%20BP (Utilities|Casting|CastToIcaroBP (Game|Player|GetPlayerPawn 0))))))
    (return)))

(fn GetHealth
  (return (.Health (Utilities|Struct|BreakSInventory (Variables|Default|GetSInventory)))))

(fn GetKeys
  (return (.Keys (Utilities|Struct|BreakSInventory (Variables|Default|GetSInventory)))))

(fn ResetHealth
  (Utilities|Struct|SetmembersinSInventory (Variables|Default|GetSInventory) 100)
  (return))

(fn ResetKeys
  (Utilities|Struct|SetmembersinSInventory (Variables|Default|GetSInventory))
  (return))