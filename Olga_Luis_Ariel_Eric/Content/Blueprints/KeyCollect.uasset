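; Collectible key pickup that the IcaroBP actor picks up by overlapping its capsule.
; The first valid overlap adds one key to MyGameInstanceBP, sets Taken and teleports the key far out of the level instead of destroying it.
; Tick also watches Taken and calls RemoveKey once to apply the same off-map move, so a key flagged as taken gets hidden.
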(event OnComponentBeginOverlap(Capsule)
  (params (OverlappedComponent :type Primitive%20Component%20Object%20Reference) (OtherActor :type Actor%20Object%20Reference) (OtherComp :type Primitive%20Component%20Object%20Reference) (OtherBodyIndex :type Integer) (bFromSweep :type Boolean) (SweepResult :type Hit%20Result%20Structure%20%28by%20ref%29))
  (Utilities|Casting|CastToIcaroBP OtherActor)
  (if (not (Variables|Default|GetTaken))
    (Utilities|FlowControl|DoOnce false
      (:Completed
        (Default|AddKeys (.AsMy%20Game%20Instance%20BP (Utilities|Casting|CastToMyGameInstanceBP (Game|GetGameInstance))) 1)
        (Variables|Default|SetTaken true)
        (Transformation|SetActorLocation "-999999.000000,-999999.000000,-999999.000000" false false)))))

(event EventTick
  (params (DeltaSeconds :type Float%20%28single-precision%29))
  (if (Variables|Default|GetTaken)
    (Utilities|FlowControl|DoOnce false
      (:Completed
        (CallFunction|RemoveKey)))))

(fn ConstructionScript)

(fn RemoveKey
  (Transformation|SetActorLocation "-999999.000000,-999999.000000,-999999.000000" false false)
  (return))