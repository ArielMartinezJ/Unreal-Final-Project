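; Demon door that opens when the player (IcaroBP) enters its trigger box and the game instance can consume the required keys.
; The requirement equals the KeyCollect actors counted at BeginPlay, displayed as text when keys are insufficient.
; Success saves OpenDoor in the game instance's inventory and plays a timeline moving the mesh along Z.
; Tick watches that flag and, once, snaps the door to its lowered open position.
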(event OnComponentBeginOverlap(Box)
  (params (OverlappedComponent :type Primitive%20Component%20Object%20Reference) (OtherActor :type Actor%20Object%20Reference) (OtherComp :type Primitive%20Component%20Object%20Reference) (OtherBodyIndex :type Integer) (bFromSweep :type Boolean) (SweepResult :type Hit%20Result%20Structure%20%28by%20ref%29))
  (bind _returnvalue (Game|GetGameInstance))
  (bind _key_number (Variables|Default|Getkey%20number))
  (bind _doorpos (Variables|Default|GetDoorPos))
  (bind (_x _y _z) (Math|Vector|BreakVector _doorpos))
  (bind _asmy_game_instance_bp (Utilities|Casting|CastToMyGameInstanceBP _returnvalue))
  (Utilities|Casting|CastToIcaroBP OtherActor)
  (if (not (Variables|Default|GetOpened))
    (bind _success (Default|ConsumeKeys _asmy_game_instance_bp (Variables|Default|GetKeyNum)))
    (if _success
      (bind _output_get (Variables|Default|SetOpened true))
      (Utilities|Struct|SetmembersinSInventory (Variables|/Game/Blueprints/Game/MyGameInstanceBP.MyGameInstanceBP_C|GetSInventory _asmy_game_instance_bp) _output_get)
      (Variables|Default|SetKeyNum 0)
      (Components|Timeline|SetPlayRate (Variables|Default|GetDoorOpening) (/ 1.0 (Variables|Default|GetTiempo%20puerta)))
      (bind _newtrack_0 (Timeline|DoorOpening PlayFromStart)
        (:Update
          (Transformation|SetRelativeLocation (Variables|Default|GetStaticMeshDemon) (Math|Vector|MakeVector _x _y (+ _z _newtrack_0)) false false)))
      (else
        (Rendering|Components|TextRender|SetText _key_number (Utilities|Text|ToText(Integer) (Variables|Default|GetKeyNum)))
        (Rendering|SetVisibility _key_number true false)))))

(event OnComponentEndOverlap(Box)
  (params (OverlappedComponent :type Primitive%20Component%20Object%20Reference) (OtherActor :type Actor%20Object%20Reference) (OtherComp :type Primitive%20Component%20Object%20Reference) (OtherBodyIndex :type Integer))
  (Utilities|Casting|CastToIcaroBP OtherActor)
  (Rendering|SetVisibility (Variables|Default|Getkey%20number) false false))

(event EventBeginPlay
  (bind _key_number (Variables|Default|Getkey%20number))
  (bind _outactors (Actor|GetAllActorsOfClass "/Game/Blueprints/KeyCollect.KeyCollect_C"))
  (for _array_element _outactors
    (Variables|Default|SetKeyNum (+ (Variables|Default|GetKeyNum) 1)))
  (Rendering|Components|TextRender|SetText _key_number (Utilities|Text|ToText(Integer) (Variables|Default|GetKeyNum)))
  (Rendering|SetVisibility _key_number false false)
  (Variables|Default|SetDoorPos (Variables|/Script/Engine.SceneComponent|GetRelativeLocation (Variables|Default|GetStaticMeshDemon))))

(event EventTick
  (params (DeltaSeconds :type Float%20%28single-precision%29))
  (bind _returnvalue (Game|GetGameInstance))
  (bind _asmy_game_instance_bp (Utilities|Casting|CastToMyGameInstanceBP _returnvalue))
  (bind _sinventory (Variables|/Game/Blueprints/Game/MyGameInstanceBP.MyGameInstanceBP_C|GetSInventory _asmy_game_instance_bp))
  (bind _opendoor (Utilities|Struct|BreakSInventory _sinventory))
  (if _opendoor
    (Rendering|SetVisibility (Variables|Default|Getkey%20number) false false)
    (Utilities|FlowControl|DoOnce false
      (:Completed
        (Variables|Default|SetOpened _opendoor)
        (CallFunction|DoorOpen)))))

(fn ConstructionScript)

(fn DoorOpen
  (bind _doorpos (Variables|Default|GetDoorPos))
  (bind (_x _y _z) (Math|Vector|BreakVector _doorpos))
  (Variables|Default|SetOpened true)
  (Variables|Default|SetKeyNum 0)
  (Transformation|SetRelativeLocation (Variables|Default|GetStaticMeshDemon) (Math|Vector|MakeVector _x _y (+ _z -3e+03)) false false)
  (return))