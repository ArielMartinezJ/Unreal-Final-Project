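; Game mode Blueprint that switches the game between main menu, in-game and pause menu states, starting at the main menu on BeginPlay.
; ChangeModeEvt routes the requested mode to its function and stores it, ignoring pause requests while already paused.
; Each function creates its widget and sets cursor and input mode.
; Entering play unpauses and removes menus; pausing pauses the game, and the main menu removes any pause menu.
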(event Custom|ChangeModeEvt
  (params (NewMode :type EGameModes%20Enum :default "NewEnumerator0"))
  (switch Utilities|FlowControl|Switch|SwitchonEGameModes NewMode
    (:NewEnumerator0
      (CallFunction|MainMnu)
      (Variables|Default|SetGameMode NewMode :!label _label))
    (:NewEnumerator1
      (CallFunction|InGame)
      (goto _label))
    (:NewEnumerator2
      (if (not (Game|IsGamePaused))
        (CallFunction|PauseMnu)
        (goto _label)))))

(event EventBeginPlay
  (CallFunction|ChangeModeEvt "NewEnumerator0"))

(fn ConstructionScript)

(fn InGame
  (bind _returnvalue (Game|GetPlayerController 0))
  (bind _pausemnuref (Variables|Default|GetPauseMnuRef))
  (bind _mainmnuwb (Variables|Default|GetMainMnuWB))
  (if (Game|IsGamePaused)
    (Game|SetGamePaused false))
  (Utilities|FlowControl|Sequence
    (:then_0
      (if (!= _mainmnuwb 0)
        (Widget|RemovefromParent _mainmnuwb))
      (Variables|/Script/Engine.PlayerController|SetbShowMouseCursor _returnvalue false)
      (Input|SetInputModeGameOnly _returnvalue)
      (bind _returnvalue_2 (UserInterface|CreateWidget "/Game/Blueprints/Game/UMG/InGameWB.InGameWB_C" (Game|GetPlayerController 0)))
      (bind _output_get (Variables|Default|SetInGameWB _returnvalue_2))
      (UserInterface|Viewport|AddtoViewport _output_get 0))
    (:then_1
      (if (!= _pausemnuref 0)
        (Widget|RemovefromParent _pausemnuref)))))

(fn MainMnu
  (bind _returnvalue (Game|GetPlayerController 0))
  (bind _pausemnuref (Variables|Default|GetPauseMnuRef))
  (if (!= _pausemnuref 0)
    (Widget|RemovefromParent _pausemnuref))
  (bind _returnvalue_2 (UserInterface|CreateWidget "/Game/Blueprints/Menu/MainMnuWB.MainMnuWB_C" (Game|GetPlayerController 0)))
  (bind _output_get (Variables|Default|SetMainMnuWB _returnvalue_2))
  (UserInterface|Viewport|AddtoViewport _output_get 0)
  (Input|SetInputModeUIOnly _returnvalue 0 "DoNotLock")
  (Variables|/Script/Engine.PlayerController|SetbShowMouseCursor _returnvalue true))

(fn PauseMnu
  (bind _returnvalue (Game|GetPlayerController 0))
  (bind _returnvalue_2 (UserInterface|CreateWidget "/Game/Blueprints/Menu/PauseMnu.PauseMnu_C" (Game|GetPlayerController 0)))
  (bind _output_get (Variables|Default|SetPauseMnuRef _returnvalue_2))
  (UserInterface|Viewport|AddtoViewport _output_get 0)
  (Game|SetGamePaused true)
  (Variables|/Script/Engine.PlayerController|SetbShowMouseCursor _returnvalue true)
  (Input|SetInputModeUIOnly _returnvalue 0 "DoNotLock"))